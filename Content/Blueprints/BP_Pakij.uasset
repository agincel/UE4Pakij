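; BP_Pakij is a Blueprint that launches its Cube component with physics impulses, steered by mouse look.
; Mouse X and Y feed yaw and inverted pitch input, scaled by MouseScale, to player pawn 0.
; Left click calls Jump, which rotates a JumpPower forward vector by that pawn's control pitch and yaw, adds JumpVerticalPower upward, and applies it as a mass-dependent impulse.
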(event `InputAxisKey|MouseX`
  (params (AxisValue :type "Float (single-precision)"))
  (`self.AddControllerYawInput` (`GameplayStatics.GetPlayerPawn` 0) (* AxisValue (`self.MouseScale`))))

(event `InputAxisKey|MouseY`
  (params (AxisValue :type "Float (single-precision)"))
  (`self.AddControllerPitchInput` (`GameplayStatics.GetPlayerPawn` 0) (* AxisValue (`self.MouseScale`) -1.0)))

(event `Key|LeftMouseButton`
  (params (Key :type "Key Structure" :default "AnyKey"))
  (:`Pressed`
    (`self.Jump`)))

(fn `Jump`
  (`PrimitiveComponent.AddImpulse` (`self.Cube`) (`KismetMathLibrary.MakeVector` (.x (`KismetMathLibrary.GreaterGreater_VectorRotator` (`KismetMathLibrary.MakeVector` (`self.JumpPower`)) (`KismetMathLibrary.MakeRotator` 0.0 (.pitch (`self.GetControlRotation` (`GameplayStatics.GetPlayerPawn` 0))) (.yaw (`self.GetControlRotation` (`GameplayStatics.GetPlayerPawn` 0)))))) (.y (`KismetMathLibrary.GreaterGreater_VectorRotator` (`KismetMathLibrary.MakeVector` (`self.JumpPower`)) (`KismetMathLibrary.MakeRotator` 0.0 (.pitch (`self.GetControlRotation` (`GameplayStatics.GetPlayerPawn` 0))) (.yaw (`self.GetControlRotation` (`GameplayStatics.GetPlayerPawn` 0)))))) (+ (.z (`KismetMathLibrary.GreaterGreater_VectorRotator` (`KismetMathLibrary.MakeVector` (`self.JumpPower`)) (`KismetMathLibrary.MakeRotator` 0.0 (.pitch (`self.GetControlRotation` (`GameplayStatics.GetPlayerPawn` 0))) (.yaw (`self.GetControlRotation` (`GameplayStatics.GetPlayerPawn` 0)))))) (`self.JumpVerticalPower`))) "None" false))

(fn `UserConstructionScript`)